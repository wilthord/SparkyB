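; Side-scrolling 2D player character with a replicated sprite, horizontal movement and jumping.
; The move axis drives X movement and flips controller yaw to face the travel direction.
; Jumping, allowed when not rising, uses high launch velocity with a short hold and arms a flag.
; While airborne, Tick consumes that flag to set a very high gravity scale; the reset to normal gravity is unconnected.
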(event `self.ReceiveBeginPlay`
  ;[1 1 1] Replication
  (`ActorComponent.SetIsReplicated` (`self.Sprite`) true))

(event `InputAxis|MoveRigth`
  (params (AxisValue :type "Float (single-precision)"))
  ;[1 1 1] Movimiento
  (`self.AddMovementInput` (1.0 0.0 0.0) AxisValue)
  (`/Engine/EditorBlueprintResources/StandardMacros.CompareFloat` AxisValue
    (:`>`
      (`Controller.SetControlRotation` (`self.GetController`) (`KismetMathLibrary.MakeRotator` 0.0)))
    (:`<`
      (`Controller.SetControlRotation` (`self.GetController`) (`KismetMathLibrary.MakeRotator` 0.0 0.0 180.0)))))

(event `InputAction|Jump`
  (params (Key :type "Key Structure" :default "AnyKey"))
  ;[1 1 1] Salto
  (:`Pressed`
    (if (<= (.z (`self.GetVelocity`)) 0.0)
      (`self.Jump`)
      (set `self.Gravedad` true)))
  (:`Released`
    (`self.StopJumping`)))

(event `self.ReceiveTick`
  (params (DeltaSeconds :type "Float (single-precision)"))
  (bind _gravedad (`self.Gravedad`))
  ;[1 1 1] Control Gravedad
  (if (`NavMovementComponent.IsFalling` (`self.CharacterMovement`))
    (`/Engine/EditorBlueprintResources/StandardMacros.CompareFloat` (.z (`self.GetVelocity`))
      (:`>`
        (if _gravedad
          (set `CharacterMovementComponent.GravityScale` 1000.0 (`self.CharacterMovement`) :!label _label)
          (set `self.Gravedad` false)))
      (:`==`
        (if _gravedad :!label _label_2
          (goto _label)))
      (:`<`
        (goto _label_2)))))

(fn `UserConstructionScript`
  (set `CharacterMovementComponent.JumpZVelocity` 10000.0 (`self.CharacterMovement`))
  (set `self.JumpMaxHoldTime` 0.3))